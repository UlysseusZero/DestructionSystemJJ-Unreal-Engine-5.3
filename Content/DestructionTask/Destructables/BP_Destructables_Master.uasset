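; Master Blueprint for destructible objects, assembled at runtime from a data table row.
; The construction script caches the row selected by RowHandleDestructable into DestructableInformation.
; On BeginPlay it spawns one BP_Destructable_Component actor per component entry, stores it and attaches it to the root.
; Each spawned piece receives its destruction fragment at layer 0, with the attach result passed as IsBaseComponent.
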(event Custom|Instantiate%20Components
  (params (Index :type Integer))
  (bind _returnvalue (Game|SpawnActorfromClass "/Game/DestructionTask/Destructables/BP_Destructable_Component.BP_Destructable_Component_C" (Transformation|GetActorTransform) "Undefined" "MultiplyWithRoot" 0 0))
  (Utilities|Array|Add (Variables|Default|GetDestructable%20Component) _returnvalue)
  (bind _returnvalue_2 (Transformation|AttachComponentToComponent _returnvalue (Variables|Default|GetDefaultSceneRoot) "None" "SnapToTarget" "SnapToTarget" "SnapToTarget" true))
  (Default|SetComponentVariable _returnvalue 0 (Utilities|Array|Get(acopy) (.components (Variables|Default|GetDestructable%20Information)) Index) _returnvalue_2))

(event EventBeginPlay
  (for (_ _array_index) (.components (Variables|Default|GetDestructable%20Information))
    (CallFunction|InstantiateComponents _array_index)))

(fn ConstructionScript
  (|CacheDestructables))