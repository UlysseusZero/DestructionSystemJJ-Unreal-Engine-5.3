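; Destructible piece actor, configured from a fragment struct with mesh, material, health, broken variants and debris meshes.
; Hits from actors passing a tag check reduce health by a fixed step and select a broken variant at low health.
; At zero health, non-base pieces clear their mesh and spawn temporary BP_Destroyed_Components debris.
; A DoOnce-gated timeline drives a dynamic material parameter to blink on hit.
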(event OnComponentHit(VisualMesh)
  (params (HitComponent :type Primitive%20Component%20Object%20Reference) (OtherActor :type Actor%20Object%20Reference) (OtherComp :type Primitive%20Component%20Object%20Reference) (NormalImpulse :type Vector :default "0, 0, 0") (Hit :type Hit%20Result%20Structure%20%28by%20ref%29))
  ;[1 1 1] On Hit Event
  (if (Actor|ActorHasTag OtherActor "None")
    (CallFunction|Damages 0.0)
    (CallFunction|Blinking)))

(event Custom|Blinking
  ;[1 1 1] Blinking Event
  (Utilities|FlowControl|DoOnce false :!label _label
    (:Completed
      (bind _newtrack_0 (Timeline|Blinking%20Timeline PlayFromStart)
        (:Update
          (Rendering|Material|SetScalarParameterValue (Variables|Default|GetDynamic%20Material) "DynamicColor" _newtrack_0 :!class /Script/Engine.MaterialInstanceDynamic))
        (:Finished
          (goto _label Reset))))))

(event Custom|Damaged
  (params (Damage :type Float%20%28double-precision%29))
  ;[1 1 1] Damaged Event
  (bind _output_get (Variables|Default|SetCurrent%20Health (Math|Float|Clamp(Float) (- (Variables|Default|GetCurrent%20Health) Damage) 0.0 (Variables|Default|GetMax%20Health))))
  (CallFunction|ChangeVisualMesh _output_get))

(event Custom|Spawn%20Destroyed%20Pieces
  ;[1 1 1] Spawn Destroyed Pieces Event
  (for _array_element (Variables|Default|GetDestroyed%20Fragments)
    (bind _returnvalue (Game|SpawnActorfromClass "/Game/DestructionTask/Destructables/BP_Destroyed_Components.BP_Destroyed_Components_C" (Transformation|GetActorTransform) "Undefined" "MultiplyWithRoot" 0 0))
    (Components|StaticMesh|SetStaticMesh (Variables|Default|GetVisualMesh) 0)
    (Default|SetDestroyedMesh _returnvalue _array_element (Variables|Default|GetDefault%20Material))
    (Actor|SetLifeSpan _returnvalue 2e+01)))

(event Custom|Change%20Visual%20Mesh
  (params (Current%20Health :type Float%20%28double-precision%29))
  ;[1 1 1] Change Visual Mesh Event
  (if (< Current%20Health (/ (Variables|Default|GetMax%20Health) (+ (Utilities|Array|Length (Variables|Default|GetBroken%20Visual%20Pieces)) 1)))
    (Components|StaticMesh|SetStaticMesh (Variables|Default|GetVisualMesh) (Utilities|Array|Get(acopy) (Variables|Default|GetBroken%20Visual%20Pieces)))
    (CallFunction|SpawnDestroyedPieces)))

(event Custom|Obliterated%20Mesh
  ;[1 1 1] Obliterated Mesh Event
  (if (<= (Variables|Default|GetCurrent%20Health) 0.0)
    (Components|StaticMesh|SetStaticMesh (Variables|Default|GetVisualMesh) 0)
    (for _array_element (Variables|Default|GetDestroyed%20Fragments)
      (bind _returnvalue (Game|SpawnActorfromClass "/Game/DestructionTask/Destructables/BP_Destroyed_Components.BP_Destroyed_Components_C" (Transformation|GetActorTransform) "Undefined" "MultiplyWithRoot" 0 0))
      (Default|SetDestroyedMesh _returnvalue _array_element (Variables|Default|GetDefault%20Material)))))

(event Custom|Set%20Component%20Variable
  (params (Layer%20Index :type Integer) (Destruction%20Fragment :type S%20Destruction%20Structure) (Is%20Base%20Component :type Boolean))
  (bind (_defaultfragment _fragmentdefaulthealth _defaultmaterial _brokenvisualpieces _destroyedfragments) (Utilities|Struct|BreakS_Destruction Destruction%20Fragment))
  ;[1 1 1] Set Component
  (Variables|Default|SetIndex Layer%20Index)
  (Components|StaticMesh|SetStaticMesh (Variables|Default|GetVisualMesh) _defaultfragment)
  (Variables|Default|SetCurrent%20Health _fragmentdefaulthealth)
  (Variables|Default|SetDefault%20Material _defaultmaterial)
  (Variables|Default|SetBroken%20Visual%20Pieces _brokenvisualpieces)
  (Variables|Default|SetDestroyed%20Fragments _destroyedfragments))

(event Custom|Damages
  (params (Damage%20Amount :type Float%20%28double-precision%29))
  (if (not (Variables|Default|GetisDestroyed))
    (if (> (- (Variables|Default|GetCurrent%20Health) Damage%20Amount) 0.0)
      (bind _output_get (Variables|Default|SetCurrent%20Health (- (Variables|Default|GetCurrent%20Health) 2.0)))
      (CallFunction|ChangeVisualsMesh _output_get)
      (elif (Variables|Default|GetisBaseComponent)
        (Variables|Default|SetCurrent%20Health 0.0)
        (else
          (Variables|Default|SetCurrent%20Health 0.0)
          (CallFunction|SpawnDestroyedPieces))))))

(event Custom|Change%20Visuals%20Mesh
  (params (Current%20Health :type Float%20%28double-precision%29))
  (bind _broken_visual_pieces (Variables|Default|GetBroken%20Visual%20Pieces))
  (if (and (< Current%20Health (/ (Variables|Default|GetMax%20Health) (+ (Utilities|Array|Length (Variables|Default|GetBroken%20Visual%20Pieces)) 1))) (> (Utilities|Array|Length (Variables|Default|GetBroken%20Visual%20Pieces)) 0))
    (Variables|Default|SetDefault%20Fragment (Utilities|Array|Get(acopy) _broken_visual_pieces (- (Utilities|Array|Length _broken_visual_pieces) 1)))))

(event EventBeginPlay
  ;[1 1 1] Event Begin Play - Dynamic Material
  (bind _returnvalue (Rendering|Material|CreateDynamicMaterialInstance (Variables|Default|GetVisualMesh) 0 (Variables|Default|GetDefault%20Material) "None" :!class /Script/Engine.PrimitiveComponent))
  (Variables|Default|SetDynamic%20Material _returnvalue))

(fn ConstructionScript)

(fn DynamicMaterial
  (Utilities|IsValid (Variables|Default|GetDynamic%20Material)
    (:Is%20Valid
      _)
    (:Is%20Not%20Valid
      (bind _returnvalue (Rendering|Material|CreateDynamicMaterialInstance (Variables|Default|GetDefault%20Material) "None" "None" :!class /Script/Engine.KismetMaterialLibrary))
      (Variables|Default|SetDynamic%20Material _returnvalue)))
  (Components|StaticMesh|SetStaticMesh (Variables|Default|GetVisualMesh) (Variables|Default|GetDefault%20Fragment))
  (Rendering|Material|SetMaterial (Variables|Default|GetVisualMesh) 0 (Variables|Default|GetDynamic%20Material)))